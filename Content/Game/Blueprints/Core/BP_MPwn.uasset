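; BP_MPwn is a networked player pawn that spawns a small BP_Ball at its Arrow, allowing one live ball at a time.
; When locally controlled, Tick passes its location through CustomEvent into NewVar and pins its Camera to the level CameraActor's transform, cached at BeginPlay outside dedicated servers.
; Non-local copies smooth their movement by interpolating toward NewVar each frame.
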(event `self.ReceiveBeginPlay`
  (set `self.NewVar` (`self.K2_GetActorLocation`))
  (if (not (`KismetSystemLibrary.IsDedicatedServer`))
    (bind _returnvalue (`GameplayStatics.GetActorOfClass` "/Script/Engine.CameraActor"))
    (set `self.NewVar_0` (`self.GetTransform` _returnvalue))))

(event `CustomEvent`
  (params (NewParam :type "Vector Structure"))
  (set `self.NewVar` NewParam))

(event `self.ReceiveTick`
  (params (DeltaSeconds :type "Float (single-precision)"))
  (bind _returnvalue (`self.K2_GetActorLocation`))
  (if (`self.IsLocallyControlled`)
    (`self.CustomEvent` _returnvalue)
    (`SceneComponent.K2_SetWorldTransform` (`self.Camera`) (`self.NewVar_0`) false false)
    (else
      (`self.K2_SetActorLocation` (`KismetMathLibrary.VInterpTo` _returnvalue (`self.NewVar`) DeltaSeconds 90.0)))))

(event `SpawnBall`
  (`self.AliveBall`
    (:`then`)
    (:`else`
      (bind _returnvalue (`|SpawnActorFromClass` "/Game/Game/Blueprints/BP_Ball.BP_Ball_C" (`KismetMathLibrary.MakeTransform` (`SceneComponent.K2_GetComponentLocation` (`self.Arrow`)) (struct) (0.1 0.1 0.1)) "Undefined" "OverrideRootScale" null false null))
      (set `self.AliveBall` _returnvalue))))

(fn `UserConstructionScript`)