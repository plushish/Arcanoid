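; Multiplayer player controller for a ball game, handling HUD, pawn input, win screen and restarts.
; Input slides the possessed BP_MPwn sideways with sweep and triggers its SpawnBall.
; Endgame shows WB_Win with UI-only input.
; ResetLvlServ counts ready players in BP_MGM; once all are ready it resets the level, cubes and score, then each controller possesses a fresh pawn at PlayerStart and returns to game input.
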(event `self.ReceiveBeginPlay`
  (if (not (`KismetSystemLibrary.IsDedicatedServer`))
    (`WidgetBlueprintLibrary.SetInputMode_GameOnly` self)
    (bind _returnvalue (`|CreateWidget` "/Game/Game/UI/WB_HUD.WB_HUD_C" self))
    (`UserWidget.AddToViewport` _returnvalue 0)))

(event `self.ReceivePossess`
  (params (PossessedPawn :type "Pawn Object Reference"))
  (bind _asbp_mpwn (cast `/Game/Game/Blueprints/Core/BP_MPwn` PossessedPawn))
  (set `self.MyPwn` _asbp_mpwn))

(event `InputAxis|Left_Right`
  (params (AxisValue :type "Float (single-precision)"))
  (bind _mypwn (`self.MyPwn`))
  (`/Engine/EditorBlueprintResources/StandardMacros.IsValid` _mypwn
    (:`Is Valid`
      (`self.K2_AddActorWorldOffset` _mypwn (`KismetMathLibrary.MakeVector` 0.0 (* AxisValue (`GameplayStatics.GetWorldDeltaSeconds`) (`self.Speed`))) true false))))

(event `InputAction|SpawnBall`
  (params (Key :type "Key Structure"))
  (:`Pressed`
    (`/Game/Game/Blueprints/Core/BP_MPwn.SpawnBall` (`self.MyPwn`))))

(event `Endgame`
  (bind _returnvalue (`|CreateWidget` "/Game/Game/UI/WB_Win.WB_Win_C" self))
  (`UserWidget.AddToViewport` _returnvalue 0)
  (`WidgetBlueprintLibrary.SetInputMode_UIOnlyEx` self _returnvalue)
  (set `self.bShowMouseCursor` true))

(event `ResetLvlServ`
  (bind _returnvalue (`GameplayStatics.GetGameMode`))
  (bind _playersready (`/Game/Game/Blueprints/Core/BP_MGM.PlayersReady` (cast `/Game/Game/Blueprints/Core/BP_MGM` (`GameplayStatics.GetGameMode`) :!pure true)))
  (`/Engine/EditorBlueprintResources/StandardMacros.IncrementInt` _playersready
    (:`  `
      (bind _outactors (`GameplayStatics.GetAllActorsOfClass` "/Script/Engine.PlayerController"))
      (if (<= (`KismetArrayLibrary.Array_Length` _outactors) _playersready)
        (set `/Game/Game/Blueprints/Core/BP_MGM.PlayersReady` 0 (cast `/Game/Game/Blueprints/Core/BP_MGM` _returnvalue :!pure true))
        (`GameModeBase.ResetLevel` _returnvalue)
        (bind _returnvalue_2 (`GameplayStatics.GetActorOfClass` "/Game/Game/Blueprints/Bp_Cube_Parrent.Bp_Cube_Parrent_C"))
        (`/Game/Game/Blueprints/Bp_Cube_Parrent.NewBeggin` _returnvalue_2)
        (set `/Game/Game/Blueprints/Bp_Cube_Parrent.ScoreCount` 0 _returnvalue_2)
        (bind _outactors_2 (`GameplayStatics.GetAllActorsOfClass` "BP_MPContr_C"))
        (for _array_element _outactors_2
          (`self.NewChar` _array_element))))))

(event `NewChar`
  (bind _returnvalue (`GameplayStatics.GetActorOfClass` "/Script/Engine.PlayerStart"))
  (bind _returnvalue_2 (`|SpawnActorFromClass` "/Game/Game/Blueprints/Core/BP_MPwn.BP_MPwn_C" (`self.GetTransform` _returnvalue) "Undefined" "OverrideRootScale" null null))
  (`self.Possess` _returnvalue_2)
  (`self.newCharOwn`))

(event `newCharOwn`
  (`WidgetBlueprintLibrary.SetInputMode_GameOnly` self)
  (set `self.bShowMouseCursor` false)
  (bind _foundwidgets (`WidgetBlueprintLibrary.GetAllWidgetsOfClass` "/Game/Game/UI/WB_Win.WB_Win_C"))
  (`Widget.RemoveFromParent` (`|GetArrayItem` _foundwidgets)))

(fn `UserConstructionScript`)