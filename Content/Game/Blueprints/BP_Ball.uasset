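; BP_Ball is a networked bouncing ball that reports hit items and locations to cube actors and reports its spawn and removal to the BP_MGM game mode's ball count.
; The server moves it with a swept offset, reflecting its direction and raising its capped speed on blocking hits, and destroys it inside trigger boxes.
; Clients smooth movement by lerping between server-recorded positions, restarting the blend on each OnRep.
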(event `self.ReceiveBeginPlay`
  (`|ExecutionSequence`
    (:`then_0`
      (if (`self.BigBall`)
        (`SceneComponent.SetRelativeScale3D` (`self.Sphere`) (0.2 0.2 0.2))))
    (:`then_1`
      (set `self.NewVar` (`self.K2_GetActorLocation`))
      (`/Engine/EditorBlueprintResources/ActorMacros.Switch Has Authority`
        (:`Authority`
          (bind _asbp_mgm (cast `/Game/Game/Blueprints/Core/BP_MGM` (`GameplayStatics.GetGameMode`)))
          (`/Game/Game/Blueprints/Core/BP_MGM.BallsCountCh` _asbp_mgm true))))))

(event `self.Sphere.OnComponentBeginOverlap`
  (params (OverlappedComponent :type "PrimitiveComponent Object Reference") (OtherActor :type "Actor Object Reference") (OtherComp :type "PrimitiveComponent Object Reference") (OtherBodyIndex :type Integer) (bFromSweep :type Boolean) (SweepResult :type "HitResult Structure (by ref)"))
  (`/Engine/EditorBlueprintResources/ActorMacros.Switch Has Authority`
    (:`Authority`
      (cast `TriggerBox` OtherActor)
      (`self.K2_DestroyActor`))))

(event `self.Sphere.OnComponentHit`
  (params (HitComponent :type "PrimitiveComponent Object Reference") (OtherActor :type "Actor Object Reference") (OtherComp :type "PrimitiveComponent Object Reference") (NormalImpulse :type "Vector Structure") (Hit :type "HitResult Structure (by ref)"))
  (bind (_bblockinghit _binitialoverlap _time _distance _location _impactpoint _normal _impactnormal _physmat _hitactor _hitcomponent _hitbonename _bonename _hititem) (`GameplayStatics.BreakHitResult` Hit))
  (bind _asbp_cube_parrent (cast `/Game/Game/Blueprints/Bp_Cube_Parrent` OtherActor))
  (`/Game/Game/Blueprints/Bp_Cube_Parrent.BallisHit` _asbp_cube_parrent _hititem _location))

(event `self.ReceiveTick`
  (params (DeltaSeconds :type "Float (single-precision)"))
  (bind (_returnvalue_x _returnvalue_y) (`KismetMathLibrary.BreakVector` (* (`self.Direction`) (* DeltaSeconds (`self.Speed`)))))
  (`|ExecutionSequence`
    (:`then_0`
      (set `self.Alpha` (+ (`self.Alpha`) (/ DeltaSeconds 0.033333)))
      (`/Engine/EditorBlueprintResources/ActorMacros.Switch Has Authority`
        (:`Authority`
          (`self.setvar` (`self.K2_GetActorLocation`)))
        (:`Remote`
          (`self.K2_SetActorLocation` (`KismetMathLibrary.VLerp` (`self.NewVar_rep`) (`self.NewVar`) (`self.Alpha`))))))
    (:`then_1`
      (`/Engine/EditorBlueprintResources/ActorMacros.Switch Has Authority`
        (:`Authority`
          (bind _sweephitresult (`self.K2_AddActorWorldOffset` (`KismetMathLibrary.MakeVector` _returnvalue_x _returnvalue_y) true))
          (bind (_bblockinghit _binitialoverlap _time _distance _location _impactpoint _normal) (`GameplayStatics.BreakHitResult` _sweephitresult))
          (if _bblockinghit
            (set `self.Direction` (`KismetMathLibrary.GetReflectionVector` (`self.Direction`) _normal))
            (set `self.Speed` (`KismetMathLibrary.FMin` (+ (`self.Speed`) (`self.Added speed`)) 2500.0))))))))

(event `self.ReceiveEndPlay`
  (params (EndPlayReason :type "EEndPlayReason Enum" :default "Destroyed"))
  (`/Engine/EditorBlueprintResources/ActorMacros.Switch Has Authority`
    (:`Authority`
      (bind _asbp_mgm (cast `/Game/Game/Blueprints/Core/BP_MGM` (`GameplayStatics.GetGameMode`)))
      (`/Game/Game/Blueprints/Core/BP_MGM.BallsCountCh` _asbp_mgm false))))

(event `setvar`
  (params (NewParam :type "Vector Structure"))
  (set `self.NewVar_rep` (`self.NewVar`))
  (set `self.NewVar` NewParam))

(fn `CustomEvent`
  (params (NewParam :type "Vector Structure")))

(fn `OnRep_NewVar`
  (set `self.Alpha` 0.0))

(fn `UserConstructionScript`)