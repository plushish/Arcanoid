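; Brick field actor for what appears to be a multiplayer brick-breaker, drawn as one instanced static mesh.
; An authority-chosen seed drives a random stream that carves gaps from a cube grid, while life and bonus values roll unseeded.
; Ball hits decrement life, then remove broken cubes, add score and sometimes spawn extra or big balls.
; An empty field calls Endgame on every BP_MPContr; NewBeggin clears and rebuilds it.
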(event `self.ReceiveBeginPlay`
  (`/Engine/EditorBlueprintResources/ActorMacros.Switch Has Authority` :!label _label
    (:`Authority`
      (set `self.Seed` (`KismetMathLibrary.RandomInteger` 2560000)))
    (:`Remote`
      _))
  (`KismetSystemLibrary.Delay` 0.2)
  (`KismetMathLibrary.SetRandomStreamSeed` (`self.Stream`) (`self.Seed`))
  (for _index (range 131)
    (for _index_2 (range 26)
      (`KismetArrayLibrary.Array_Add` (`self.Array`) (`KismetMathLibrary.MakeTransform` (`KismetMathLibrary.MakeVector` (`KismetMathLibrary.Conv_IntToDouble` (* _index 100)) (`KismetMathLibrary.Conv_IntToDouble` (* _index_2 100)))))))
  (for _ (range 2001)
    (bind _output_get (set `self.buff` (`KismetMathLibrary.RandomIntegerInRangeFromStream` 0 (`KismetArrayLibrary.Array_LastIndex` (`self.Array`)) (`self.Stream`))))
    (`KismetArrayLibrary.Array_Remove` (`self.Array`) _output_get))
  (for _ (range (+ (`KismetArrayLibrary.Array_LastIndex` (`self.Array`)) 1))
    (`KismetArrayLibrary.Array_Add` (`self.Life`) (`KismetMathLibrary.RandomIntegerInRange` 0 1))
    (`KismetArrayLibrary.Array_Add` (`self.Bonus`) (`KismetMathLibrary.RandomIntegerInRange` 0 50)))
  (for _array_element (`self.Array`)
    (`InstancedStaticMeshComponent.AddInstance` (`self.InstancedStaticMesh`) _array_element false)))

(event `NewBeggin`
  (`KismetArrayLibrary.Array_Clear` (`self.Life`))
  (`KismetArrayLibrary.Array_Clear` (`self.Bonus`))
  (`KismetArrayLibrary.Array_Clear` (`self.Array`))
  (`InstancedStaticMeshComponent.ClearInstances` (`self.InstancedStaticMesh`))
  (goto _label))

(event `BallisHit`
  (params (IndexHit :type Integer) (PlaceHit :type "Vector Structure"))
  (bind _life (`self.Life`))
  (bind _returnvalue (- (`|GetArrayItem` _life IndexHit) 1))
  (`KismetArrayLibrary.Array_Set` _life IndexHit _returnvalue)
  (if (<= _returnvalue 0)
    (switch `int` (`|GetArrayItem` (`self.Bonus`) IndexHit)
      (:`Default`
        _)
      (:`0`
        (`|SpawnActorFromClass` "/Game/Game/Blueprints/BP_Ball.BP_Ball_C" (`KismetMathLibrary.MakeTransform` PlaceHit (struct) (0.1 0.1 0.1)) "Undefined" "OverrideRootScale" null false null)
        (`|SpawnActorFromClass` "/Game/Game/Blueprints/BP_Ball.BP_Ball_C" (`KismetMathLibrary.MakeTransform` (+ PlaceHit (0.0 0.0 0.0)) (struct) (0.1 0.1 0.1)) "Undefined" "OverrideRootScale" null false null))
      (:`1`
        (`|SpawnActorFromClass` "/Game/Game/Blueprints/BP_Ball.BP_Ball_C" (`KismetMathLibrary.MakeTransform` PlaceHit (struct) (0.1 0.1 0.1)) "Undefined" "OverrideRootScale" null true null)))
    (set `self.ScoreCount` (+ (`self.ScoreCount`) 100))
    (`self.BallsHitMulti` IndexHit)
    (if (<= (`InstancedStaticMeshComponent.GetInstanceCount` (`self.InstancedStaticMesh`)) 0)
      (bind _outactors (`GameplayStatics.GetAllActorsOfClass` "/Game/Game/Blueprints/Core/BP_MPContr.BP_MPContr_C"))
      (for _array_element _outactors
        (`/Game/Game/Blueprints/Core/BP_MPContr.Endgame` _array_element)))))

(event `BallsHitMulti`
  (params (NewParam :type Integer))
  (`InstancedStaticMeshComponent.RemoveInstance` (`self.InstancedStaticMesh`) NewParam))

(fn `UserConstructionScript`)

(fn `WinCondition`
  (if (<= (`InstancedStaticMeshComponent.GetInstanceCount` (`self.InstancedStaticMesh`)) 0)
    _))